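; Launch pad that throws an overlapping Ue4ASP_Character straight upward, with a height set by how many linked buttons are active.
; Activation and deactivation events keep separate counts for buttons and sub-buttons.
; On overlap, the sub-button count is subtracted from the button count, clamped to a small range, and scaled onto a base vertical velocity passed to LaunchCharacter.
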(event EventBeginPlay)

(event EventSubButtonActivated
  ;[1 1 1] Increment/Decrement Button Count
  (bind _result (Math|Integer|IncrementInt (Variables|Default|GetSubButtonPressed))
    (:%20%20
      (Variables|Default|SetSubButtonPressed _result))))

(event EventSubButtonDeactivated
  ;[1 1 1] Increment/Decrement Button Count
  (bind _result (Math|Integer|DecrementInt (Variables|Default|GetSubButtonPressed))
    (:%20%20
      (Variables|Default|SetSubButtonPressed _result))))

(event EventTick
  (params (DeltaSeconds :type Float%20%28single-precision%29)))

(event Collision|EventActorBeginOverlap
  (params (OtherActor :type Actor%20Object%20Reference))
  (bind _asue_4asp_character (Utilities|Casting|CastToUe4ASP_Character OtherActor))
  (Character|LaunchCharacter _asue_4asp_character (Math|Conversions|ToVector(Float) (Utilities|Struct|MakeIntVector 0 0 (+ (* (Math|Integer|Clamp(Integer) (- (Variables|Default|GetButtonsPressed) (Variables|Default|GetSubButtonPressed)) 0 4) 147) 1033))) false false))

(event EventButtonActivated
  ;[1 1 1] Increment/Decrement Button Count
  (bind _result (Math|Integer|IncrementInt (Variables|Default|GetButtonsPressed))
    (:%20%20
      (Variables|Default|SetButtonsPressed _result))))

(event EventButtonDeactivated
  ;[1 1 1] Increment/Decrement Button Count
  (bind _result (Math|Integer|DecrementInt (Variables|Default|GetButtonsPressed))
    (:%20%20
      (Variables|Default|SetButtonsPressed _result))))

(fn ConstructionScript)